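; DamageField_BP is an area trigger that repeatedly damages a ThirdPersonCharacter1 inside its Box component.
; Begin overlap casts the actor and starts a Delay-based loop that applies the Damage and DamageType variables every 0.01 seconds while the Overlap flag is set.
; The loop only deals damage while Health is 99 or below; higher Health clears the flag.
; Any end overlap also clears the flag, regardless of which actor leaves.
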(event `self.Box.OnComponentBeginOverlap`
  (params (OverlappedComponent :type "PrimitiveComponent Object Reference") (OtherActor :type "Actor Object Reference") (OtherComp :type "PrimitiveComponent Object Reference") (OtherBodyIndex :type Integer) (bFromSweep :type Boolean) (SweepResult :type "HitResult Structure (by ref)"))
  (set `self.Overlap` true)
  (bind _asthird_person_character_1 (cast `/Game/ThirdPersonBP/Blueprints/ThirdPersonCharacter1` OtherActor))
  (bind _health (`/Game/ThirdPersonBP/Blueprints/ThirdPersonCharacter1.Health` _asthird_person_character_1))
  (set `/Game/ThirdPersonBP/Blueprints/ThirdPersonCharacter1.Health` _health _asthird_person_character_1)
  (if (<= _health 99) :!label _label
    (if (`self.Overlap`)
      (`GameplayStatics.ApplyDamage` _asthird_person_character_1 (`self.Damage`) null null "/Script/Engine.DamageType")
      (`KismetSystemLibrary.Delay` 0.01)
      (goto _label))
    (else
      (set `self.Overlap` false))))

(event `self.Box.OnComponentEndOverlap`
  (params (OverlappedComponent :type "PrimitiveComponent Object Reference") (OtherActor :type "Actor Object Reference") (OtherComp :type "PrimitiveComponent Object Reference") (OtherBodyIndex :type Integer))
  (set `self.Overlap` false))

(fn `UserConstructionScript`)