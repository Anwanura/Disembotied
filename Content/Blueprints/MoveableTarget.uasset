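; MoveableTarget is a boomerang target that slides along Y on a timeline and explodes when hit enough.
; Each Boomerang overlap raises TransitionValue on a dynamic material, and reaching the threshold sets MaterialChanged.
; The timeline update watches that flag, then after a short delay plays explosion effects and destroys the actor.
; On destruction it asks SpawnerRef to spawn at its location, passing along its movement range.
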(event `self.ReceiveBeginPlay`
  (bind _staticmesh (`self.StaticMesh`))
  (bind _returnvalue (`PrimitiveComponent.CreateDynamicMaterialInstance` _staticmesh 0 (`PrimitiveComponent.GetMaterial` _staticmesh 0)))
  (bind (_direction _newtrack_0) (`Timeline|Movement`)
    (:`Update`
      (`SceneComponent.K2_SetRelativeLocation` (`self.StaticMesh`) (`KismetMathLibrary.MakeVector` 0.0 (`KismetMathLibrary.Lerp` (`self.StartY`) (`self.EndY`) _newtrack_0)) false false)
      (if (`self.MaterialChanged`)
        (`KismetSystemLibrary.Delay` 0.3)
        (`GameplayStatics.PlaySoundAtLocation` "/Game/StarterContent/Audio/Explosion_Cue.Explosion_Cue" (`self.K2_GetActorLocation`) (`self.K2_GetActorRotation`))
        (`GameplayStatics.SpawnEmitterAtLocation` "/Game/StarterContent/Particles/P_Explosion.P_Explosion" (`SceneComponent.K2_GetComponentLocation` (`self.StaticMesh`)))
        (`self.K2_DestroyActor`)))))

(event `self.ReceiveDestroyed`
  (`/Game/Blueprints/BP_TargetSpawner.Spawn` (`self.SpawnerRef`) (`self.StartY`) (`self.EndY`) (`self.K2_GetActorLocation`) (`self.K2_GetActorRotation`)))

(event `self.Box.OnComponentBeginOverlap`
  (params (OverlappedComponent :type "PrimitiveComponent Object Reference") (OtherActor :type "Actor Object Reference") (OtherComp :type "PrimitiveComponent Object Reference") (OtherBodyIndex :type Integer) (bFromSweep :type Boolean) (SweepResult :type "HitResult Structure (by ref)"))
  (cast `/Game/ThirdPersonBP/Blueprints/Boomerang` OtherActor)
  (if (`self.ChangeMaterial`)
    _
    (else
      _))
  (bind _returnvalue (`MaterialInstanceDynamic.K2_GetScalarParameterValue` (`self.Material`) (`self.TransitionValue`)))
  (bind _returnvalue_2 (+ _returnvalue 5.0))
  (`MaterialInstanceDynamic.SetScalarParameterValue` (stale `self.ReceiveBeginPlay` _returnvalue) "TransitionValue" _returnvalue_2)
  (if (>= _returnvalue_2 10.0)
    (set `self.MaterialChanged` true)))

(fn `UserConstructionScript`
  (bind _returnvalue (`PrimitiveComponent.CreateDynamicMaterialInstance` (`self.StaticMesh`) 0 "/Game/Materials/M_TargetTrans.M_TargetTrans"))
  (set `self.Material` _returnvalue))