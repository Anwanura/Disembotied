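; Two-way teleporter actor that moves the player pawn between two linked points.
; Overlapping either trigger, Tele1 or Tele2, moves player 0's pawn to an arrow's location (Arrow2 and Arrow respectively) without checking which actor overlapped.
; Both paths play a shared teleport sound.
; On BeginPlay it assigns the sound cues and starts the portal audio on both portal audio components.
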(event `self.Tele1.OnComponentBeginOverlap`
  (params (OverlappedComponent :type "PrimitiveComponent Object Reference") (OtherActor :type "Actor Object Reference") (OtherComp :type "PrimitiveComponent Object Reference") (OtherBodyIndex :type Integer) (bFromSweep :type Boolean) (SweepResult :type "HitResult Structure (by ref)"))
  (`self.K2_SetActorLocation` (`GameplayStatics.GetPlayerPawn` 0) (`SceneComponent.K2_GetComponentLocation` (`self.Arrow2`)) false false)
  (`AudioComponent.Play` (`self.Teleport`) 0.0 :!label _label))

(event `self.ReceiveBeginPlay`
  (`AudioComponent.SetSound` (`self.Teleport`) "/Game/Sound/Teleport_cue.Teleport_cue")
  (`AudioComponent.SetSound` (`self.Portal_cue`) "/Game/Sound/Portal_cue.Portal_cue")
  (`AudioComponent.SetSound` (`self.Portal_cue2`) "/Game/Sound/Portal_cue.Portal_cue")
  (`AudioComponent.Play` (`self.Portal_cue`) 0.0)
  (`AudioComponent.Play` (`self.Portal_cue2`) 0.0))

(event `self.Tele2.OnComponentBeginOverlap`
  (params (OverlappedComponent :type "PrimitiveComponent Object Reference") (OtherActor :type "Actor Object Reference") (OtherComp :type "PrimitiveComponent Object Reference") (OtherBodyIndex :type Integer) (bFromSweep :type Boolean) (SweepResult :type "HitResult Structure (by ref)"))
  (`self.K2_SetActorLocation` (`GameplayStatics.GetPlayerPawn` 0) (`SceneComponent.K2_GetComponentLocation` (`self.Arrow`)) false false)
  (goto _label))

(fn `UserConstructionScript`)