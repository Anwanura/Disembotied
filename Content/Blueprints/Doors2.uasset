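; Door Blueprint that swings open only while both of its pressure triggers are overlapped.
; Begin and end overlaps on Trigger and Trigger2 set a flag for each, and their AND decides whether the Movement timeline plays or reverses.
; The timeline lerps the Arrow component's yaw through a quarter turn, so leaving either trigger swings it back.
; Overlaps are not filtered by actor or counted.
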(event `self.Trigger2.OnComponentBeginOverlap`
  (params (OverlappedComponent :type "PrimitiveComponent Object Reference") (OtherActor :type "Actor Object Reference") (OtherComp :type "PrimitiveComponent Object Reference") (OtherBodyIndex :type Integer) (bFromSweep :type Boolean) (SweepResult :type "HitResult Structure (by ref)"))
  (bind _output_get (set `self.PressureTrigger2` true))
  (set `self.Pressure` (and _output_get (stale `self.Trigger.OnComponentBeginOverlap` _output_get)) :!label _label)
  (if (`self.Pressure`)
    (bind (_direction _newtrack_0) (`Timeline|movement` :!label _label_2)
      (:`Update`
        (`SceneComponent.K2_SetRelativeRotation` (`self.Arrow`) (`KismetMathLibrary.MakeRotator` 0.0 0.0 (`KismetMathLibrary.Lerp` 0.0 -90.0 _newtrack_0)) false false)))))

(event `self.Trigger.OnComponentBeginOverlap`
  (params (OverlappedComponent :type "PrimitiveComponent Object Reference") (OtherActor :type "Actor Object Reference") (OtherComp :type "PrimitiveComponent Object Reference") (OtherBodyIndex :type Integer) (bFromSweep :type Boolean) (SweepResult :type "HitResult Structure (by ref)"))
  (bind _output_get (set `self.PressureTrigger` true))
  (goto _label))

(event `self.Trigger2.OnComponentEndOverlap`
  (params (OverlappedComponent :type "PrimitiveComponent Object Reference") (OtherActor :type "Actor Object Reference") (OtherComp :type "PrimitiveComponent Object Reference") (OtherBodyIndex :type Integer))
  (bind _output_get (set `self.PressureTrigger2` false))
  (set `self.Pressure` (and _output_get (stale `self.Trigger.OnComponentEndOverlap` _output_get)) :!label _label_3)
  (if (not (`self.Pressure`))
    (goto _label_2 :!via `Reverse`)))

(event `self.Trigger.OnComponentEndOverlap`
  (params (OverlappedComponent :type "PrimitiveComponent Object Reference") (OtherActor :type "Actor Object Reference") (OtherComp :type "PrimitiveComponent Object Reference") (OtherBodyIndex :type Integer))
  (bind _output_get (set `self.PressureTrigger` false))
  (goto _label_3))

(fn `UserConstructionScript`)