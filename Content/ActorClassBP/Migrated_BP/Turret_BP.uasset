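; Turret that tracks whatever actor last entered its trigger box and fires projectiles at it.
; Overlap plays a portal sound, spawns an emitter and activates the turret after a short delay; the stored target leaving deactivates it.
; While active, Tick interpolates the Arrow toward the target and spawns Projectile_BP from the Projectile component's transform, using a resettable DoOnce and Delay to set fire rate.
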(event `self.Box.OnComponentBeginOverlap`
  (params (OverlappedComponent :type "PrimitiveComponent Object Reference") (OtherActor :type "Actor Object Reference") (OtherComp :type "PrimitiveComponent Object Reference") (OtherBodyIndex :type Integer) (bFromSweep :type Boolean) (SweepResult :type "HitResult Structure (by ref)"))
  ;[1 1 1] Turret aggros when the player enters the triggerbox
  (set `self.Actor` OtherActor)
  (`GameplayStatics.SpawnSoundAtLocation` (`self.Portal Sound`) (`SceneComponent.K2_GetComponentLocation` (`self.Arrow`)))
  (`GameplayStatics.SpawnEmitterAtLocation` null (`SceneComponent.K2_GetComponentLocation` (`self.Billboard`)) (struct))
  (`/Engine/EditorBlueprintResources/StandardMacros.DoOnce` false :!label _label
    (:`Completed`
      (`KismetSystemLibrary.Delay` 2.0)
      (set `self.Activate` true))))

(event `self.Box.OnComponentEndOverlap`
  (params (OverlappedComponent :type "PrimitiveComponent Object Reference") (OtherActor :type "Actor Object Reference") (OtherComp :type "PrimitiveComponent Object Reference") (OtherBodyIndex :type Integer))
  ;[1 1 1] Turret stops when the player leaves the triggerbox
  (if (== OtherActor (`self.Actor`))
    (set `self.Activate` false)
    (goto _label :!via `Reset`)))

(event `self.ReceiveTick`
  (params (DeltaSeconds :type "Float (single-precision)"))
  (bind _arrow (`self.Arrow`))
  ;[1 1 1] Turret follows the player while in the triggerbox
  (if (`self.Activate`)
    (`SceneComponent.K2_SetWorldRotation` (`self.Arrow`) (`KismetMathLibrary.RInterpTo` (`SceneComponent.K2_GetComponentRotation` _arrow) (`KismetMathLibrary.FindLookAtRotation` (`SceneComponent.K2_GetComponentLocation` _arrow) (`self.K2_GetActorLocation` (`self.Actor`))) DeltaSeconds (`self.Track_Speed`)) false false)
    ;[1 1 1] Projectile shoots when the player enters the box range
    (`/Engine/EditorBlueprintResources/StandardMacros.DoOnce` false :!label _label_2
      (:`Completed`
        (`GameplayStatics.SpawnSoundAtLocation` (`self.ProjectileShot`) (`self.K2_GetActorLocation`))
        (`|SpawnActorFromClass` "/Game/ActorClassBP/Migrated_BP/Projectile_BP.Projectile_BP_C" (`SceneComponent.K2_GetComponentToWorld` (`self.Projectile`)) "AlwaysSpawn" "OverrideRootScale")
        (`KismetSystemLibrary.Delay` (`self.Fire Rate`))
        (goto _label_2 :!via `Reset`)))))

(fn `UserConstructionScript`)