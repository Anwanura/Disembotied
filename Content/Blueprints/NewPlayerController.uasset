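; Player controller Blueprint that switches the player between pawns with the Tab key.
; Each press advances an index through a pawn array, wrapping around with modulo, and makes player controller 0 possess the pawn at that index.
; The construction script is empty, and nothing in this file fills the pawn array.
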(event `Key|Tab`
  (params (Key :type "Key Structure" :default "AnyKey"))
  (:`Pressed`
    (set `self.Pawn Index` (mod (+ (`self.Pawn Index`) 1) (`KismetArrayLibrary.Array_Length` (`self.Pawn Array`))))
    (`self.Possess` (`GameplayStatics.GetPlayerController` 0) (`KismetArrayLibrary.Array_Get` (`self.Pawn Array`) (`self.Pawn Index`)))))

(fn `UserConstructionScript`)